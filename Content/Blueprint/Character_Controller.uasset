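; Character_Controller Blueprint that owns a custom on-screen notification widget and controls when it is visible.
; On BeginPlay it creates the widget, adds it to the viewport, enables the mouse cursor with Game and UI input, then hides it.
; HiddenUI toggles the widget between hidden and hit-test-invisible, stopping or playing its sped-up notification animation.
; A playing flag keeps repeated show calls from restarting the animation.
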(event `self.ReceiveBeginPlay`
  (`self.CreateCustomUI`)
  (`self.HiddenUI` true))

(event `self.ReceiveTick`
  (params (DeltaSeconds :type "Float (single-precision)")))

(fn `CreateCustomUI`
  (bind _returnvalue (`GameplayStatics.GetPlayerController` 0))
  (bind _returnvalue_2 (`|CreateWidget` "/Game/Widget/CumtomWidget.CumtomWidget_C"))
  (bind _output_get (set `self.CustomWidget` _returnvalue_2))
  (`UserWidget.AddToViewport` _output_get 0)
  (set `PlayerController.bShowMouseCursor` true _returnvalue)
  (`WidgetBlueprintLibrary.SetInputMode_GameAndUIEx` _returnvalue null))

(fn `HiddenUI`
  (params (Hide :type Boolean))
  (bind _customwidget (`self.CustomWidget`))
  (bind _notification_anim (`/Game/Widget/CumtomWidget.Notification_Anim` _customwidget))
  (if Hide
    (`Widget.SetVisibility` _customwidget "Hidden")
    (`UserWidget.StopAnimation` _customwidget _notification_anim)
    (set `self.Hidden UI Playing` false)
    (elif (not (`self.Hidden UI Playing`))
      (`Widget.SetVisibility` _customwidget "HitTestInvisible")
      (`UserWidget.PlayAnimation` _customwidget _notification_anim 0.0 1 "Forward" 3.0 false)
      (set `self.Hidden UI Playing` true))))

(fn `UserConstructionScript`)