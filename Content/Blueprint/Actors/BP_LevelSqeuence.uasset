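; Level sequence director actor that plays the cinematics around the Omega character's customization phase and hands off to battle.
; BeginPlay creates a sequence player, flags the character as customizing, plays the first frame range with input disabled, then shows the controller's UI.
; Event_OffCustomize removes that UI, hides the character, plays a later range, then starts battle, repositions the character and creates the in-game UI.
; Delays time each handoff; CInePause skips it once.
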(event `self.ReceiveBeginPlay`
  (bind _returnvalue (`GameplayStatics.GetPlayerController` 0))
  (bind _sequenceplayer (`self.SequencePlayer`))
  ;[1 1 1] Level Sequence 생성
  (bind _outactor (`LevelSequencePlayer.CreateLevelSequencePlayer` (`self.Sequence`) (make `MovieSceneSequencePlaybackSettings` false (struct) 1.0 0.0 false true false false false false false true)))
  (bind _output_get (set `self.SequencePlayer` (`LevelSequenceActor.SequencePlayer` _outactor)))
  (set `self.SequenceReference` _output_get)
  (bind _asbp_omega_character (cast `/Game/Blueprint/Character/BP_Omega_Character` (`GameplayStatics.GetPlayerCharacter` 0)))
  (bind _output_get_2 (set `/Game/Blueprint/Character/BP_Omega_Character.OnCustomize` true _asbp_omega_character))
  (set `self.LS_OnCustomize` _output_get_2)
  (`|ExecutionSequence`
    (:`then_0`
      ;[1 1 1] 캐릭터의 컨트롤러와 폰을 미리 저장
      (set `self.MyController` _returnvalue)
      (set `self.MyPawn` (`Controller.K2_GetPawn` _returnvalue)))
    (:`then_1`
      (`self.DisableInput` (`self.MyPawn`) (`self.MyController`))
      ;[1 1 1] 시퀀스 플레이
      (`MovieSceneSequencePlayer.SetFrameRange` _sequenceplayer 0 480 0.0)
      (`MovieSceneSequencePlayer.Play` _sequenceplayer)
      ;[1 1 1] 시퀀스 재생 시간 동안 딜레이
      (`KismetSystemLibrary.Delay` (`TimeManagementBlueprintLibrary.Conv_QualifiedFrameTimeToSeconds` (`MovieSceneSequencePlayer.GetDuration` (`self.SequenceReference`))))
      ;[1 1 1] 플레이어 재작동
      (`MovieSceneSequencePlayer.Stop` (`self.SequenceReference`))
      (`self.EnableInput` (`self.MyPawn`) (`self.MyController`))
      (if (`self.CIne_Pause`)
        (set `self.CIne_Pause` false)
        (else
          (bind _ascharacter_controller (cast `/Game/Blueprint/Character_Controller` _returnvalue))
          (`/Engine/EditorBlueprintResources/StandardMacros.IsValid` _ascharacter_controller
            (:`Is Valid`
              (`/Game/Blueprint/Character_Controller.HiddenUI` _ascharacter_controller false "Forward"))))))))

(event `Event_OffCustomize`
  (bind _mycontroller (`self.MyController`))
  (bind _sequenceplayer (`self.SequencePlayer`))
  (set `self.LS_OnCustomize` false)
  ;[1 1 1] UI  애니메이션  & 삭제
  (bind _ascharacter_controller (cast `/Game/Blueprint/Character_Controller` (`self.MyController`)))
  (`/Engine/EditorBlueprintResources/StandardMacros.IsValid` _ascharacter_controller
    (:`Is Valid`
      (set `/Game/Blueprint/Character_Controller.UI Playing` false _ascharacter_controller)
      (`/Game/Blueprint/Character_Controller.HiddenUI` _ascharacter_controller false "Reverse")
      ;[1 1 1] 입력 정지
      (`self.DisableInput` (`self.MyPawn`) (`self.MyController`))
      (`KismetSystemLibrary.Delay` (- (`WidgetAnimation.GetEndTime` (`/Game/Widget/CumtomWidget.Notification_Anim` (`/Game/Blueprint/Character_Controller.CustomWidget` _ascharacter_controller))) 1.5))
      (`/Game/Blueprint/Character_Controller.DeleteCustomWidget` _ascharacter_controller)
      (bind _asbp_omega_character (cast `/Game/Blueprint/Character/BP_Omega_Character` (`self.MyPawn`)))
      (`SceneComponent.SetVisibility` (`Actor.RootComponent` _asbp_omega_character) false true)
      (`MovieSceneSequencePlayer.SetFrameRange` _sequenceplayer 510 315 0.0)
      (`MovieSceneSequencePlayer.Play` _sequenceplayer)
      (`KismetSystemLibrary.Delay` (`TimeManagementBlueprintLibrary.Conv_QualifiedFrameTimeToSeconds` (`MovieSceneSequencePlayer.GetDuration` (`self.SequenceReference`))))
      (`MovieSceneSequencePlayer.Stop` (`self.SequenceReference`))
      ;[1 1 1] 입력 활성화
      (`self.EnableInput` (`self.MyPawn`) (`self.MyController`))
      (if (`self.CIne_Pause`)
        (set `self.CIne_Pause` false)
        (else
          (bind _asbp_omega_character_2 (cast `/Game/Blueprint/Character/BP_Omega_Character` (`self.MyPawn`)))
          (`/Game/Blueprint/Character/BP_Omega_Character.Event_BattleStart` _asbp_omega_character_2)
          (bind _rootcomponent (`Actor.RootComponent` _asbp_omega_character_2))
          (`SceneComponent.K2_SetWorldLocation` _rootcomponent (948.04071 1900.0 98.041496) false false)
          (`SceneComponent.SetVisibility` _rootcomponent true true)
          ;[1 1 1] InGame UI생성
          (bind _ascharacter_controller_2 (cast `/Game/Blueprint/Character_Controller` (`self.MyController`)))
          (`/Engine/EditorBlueprintResources/StandardMacros.IsValid` _ascharacter_controller_2
            (:`Is Valid`
              (`/Game/Blueprint/Character_Controller.CreateInGameUI` _ascharacter_controller_2)
              (set `PlayerController.bShowMouseCursor` false _mycontroller)
              (`WidgetBlueprintLibrary.SetInputMode_GameOnly` _mycontroller))))))))

(fn `UserConstructionScript`)