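; BP_Hitbox is an attack hitbox actor that damages any BP_Omega_Character that begins overlapping it.
; On overlap it calls DamageChar on that character, passing its own location as the damage position and its AttackType as the damage type.
; The construction script gives the HitBox component a light or heavy material based on AttackType.
; A hit-debug chain that temporarily hides the box and disables collision is unconnected and never runs.
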(event `self.ReceiveActorBeginOverlap`
  (params (OtherActor :type "Actor Object Reference"))
  (bind _asbp_omega_character (cast `/Game/Blueprint/Character/BP_Omega_Character` OtherActor))
  (`/Game/Blueprint/Character/BP_Omega_Character.Damage_Char` _asbp_omega_character (`self.K2_GetActorLocation`) (`self.AttackType`)))

(fn `UserConstructionScript`
  (bind _hitbox (`self.HitBox`))
  (if (== (`self.AttackType`) 0)
    (`PrimitiveComponent.SetMaterial` _hitbox 0 "/Game/EssentialSwordShieldAnimations/Material/MI_Hitbox_Light.MI_Hitbox_Light")
    (else
      (`PrimitiveComponent.SetMaterial` _hitbox 0 "/Game/EssentialSwordShieldAnimations/Material/MI_Hitbox_Heavy.MI_Hitbox_Heavy"))))