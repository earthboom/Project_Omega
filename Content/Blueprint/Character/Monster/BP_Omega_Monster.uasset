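; Omega monster Blueprint that carries an ornate axe, randomly picks its attacks and can chase the player.
; The construction script sets the scaled axe mesh on WeaponSocket.
; A random stream, seeded on BeginPlay, chooses combo or non-combo and an attack index, re-rolled through AttackRandomValueEvent.
; TraceToPlayer runs AI MoveTo toward the player's pawn, prints debug status and retries after a delay on success or failure; nothing here starts it.
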(event `self.ReceiveTick`
  (params (DeltaSeconds :type "Float (single-precision)")))

(event `self.ReceiveBeginPlay`
  (`KismetMathLibrary.SeedRandomStream` (`self.RandomValue`))
  (`self.AttackRandomValueFunction`))

(event `AttackRandomValueEvent`
  (`self.AttackRandomValueFunction`))

(event `TraceToPlayer`
  (bind _movementresult (`|AIMoveTo` (`Controller.K2_GetPawn` (`self.GetController`)) (0.0 0.0 0.0) (`Controller.K2_GetPawn` (`GameplayStatics.GetPlayerController` 0)) 10.0 true)
    (:`then`
      (bind _returnvalue (`|GetEnumeratorNameAsString` _movementresult))
      (`KismetSystemLibrary.PrintString` (`KismetStringLibrary.Concat_StrStr` _returnvalue ", 실행")))
    (:`OnSuccess`
      (`KismetSystemLibrary.PrintString` (`KismetStringLibrary.Concat_StrStr` _returnvalue ", 성공") true true (struct :`R` 1.0 :`A` 1.0))
      (`KismetSystemLibrary.Delay` 3.0 :!label _label)
      (`self.TraceToPlayer`))
    (:`OnFail`
      (`KismetSystemLibrary.PrintString` (`KismetStringLibrary.Concat_StrStr` _returnvalue ", 실패") true true (struct :`R` 0.007855 :`G` 1.0 :`A` 1.0))
      (goto _label))))

(fn `AttackRandomValueFunction`
  (bind _randomvalue (`self.RandomValue`))
  (bind _returnvalue (`KismetMathLibrary.RandomIntegerInRangeFromStream` 0 4 _randomvalue))
  (bind _output_get (set `self.isCombo` (`KismetMathLibrary.RandomBoolFromStream` _randomvalue)))
  (if _output_get
    (set `self.ComboNum` _returnvalue)
    (else
      (bind _output_get_2 (set `self.NoComboNum` _returnvalue))
      (`KismetSystemLibrary.PrintString` (`KismetStringLibrary.Concat_StrStr` "NoCombo Num  : " (`KismetStringLibrary.Conv_IntToString` _output_get_2))))))

(fn `UserConstructionScript`
  (bind _weaponsocket (`self.WeaponSocket`))
  (`StaticMeshComponent.SetStaticMesh` _weaponsocket "/Game/Mesh/Weapons/SM_Wep_Ornate_Axe_02.SM_Wep_Ornate_Axe_02")
  (`SceneComponent.SetRelativeScale3D` _weaponsocket (1.5 1.5 1.5)))