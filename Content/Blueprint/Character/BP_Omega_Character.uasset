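; Player character Blueprint for third-person melee action, with an OnCustomize mode where mouse-drag spins the mesh instead of moving or attacking.
; Tick eases spring-arm zoom, interpolates walk, jog and hold-to-run speeds, and snaps rotation toward control yaw on request.
; Inputs and Damage events set attack, dodge, hit and local-direction state, cleared by Reset events.
; Mesh and weapon/shield loadouts come from indexed arrays; temporary keys cycle meshes and drain HP or stamina.
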(event `self.ReceiveTick`
  (params (DeltaSeconds :type "Float (single-precision)"))
  (bind _returnvalue (`GameplayStatics.GetWorldDeltaSeconds`))
  (bind _springarm (`self.SpringArm`))
  (bind _charactermovement (`self.CharacterMovement`))
  (bind _maxwalkspeed (`CharacterMovementComponent.MaxWalkSpeed` _charactermovement))
  ;[1 1 1] Tick
  (`|ExecutionSequence`
    (:`then_0`
      ;;[1 1 1] 스무스 카메라 (스프링 암 이용)
      (if (!= (`SpringArmComponent.TargetArmLength` (`self.SpringArm`)) (`self.OriginArmLength`))
        (set `SpringArmComponent.TargetArmLength` (`KismetMathLibrary.Lerp` (`SpringArmComponent.TargetArmLength` _springarm) (`self.OriginArmLength`) (* DeltaSeconds 2.0)) _springarm)))
    (:`then_1`
      (set `CharacterMovementComponent.bOrientRotationToMovement` true _charactermovement)
      (if (`self.IsSnapRotation`)
        (`self.SnapRotationFn`
          (:`Output`
            _)))
      (if (and (`self.isHoldShift`) (`self.isLocomotion`))
        (`/Engine/EditorBlueprintResources/StandardMacros.IncrementInt` (`self.pre_RunTimer`)
          (:`  `
            (if (> (`self.pre_RunTimer`) 20)
              (set `self.isRun` true)
              ;;[1 1 1] Set Rotation rate
              (set `CharacterMovementComponent.RotationRate` (struct :`Yaw` 540.0) _charactermovement)
              ;;[1 1 1] Set Movement Speed
              (set `CharacterMovementComponent.MaxWalkSpeed` (`KismetMathLibrary.FInterpTo` _maxwalkspeed (`self.Speed_Run`) _returnvalue 10.0) _charactermovement)
              (`/Engine/EditorBlueprintResources/StandardMacros.IncrementInt` (`self.RunTimer`)))))
        (else
          (set `self.isRun` false)
          (set `CharacterMovementComponent.RotationRate` (struct :`Yaw` 540.0) _charactermovement)
          (if (`self.isWalk`)
            (set `CharacterMovementComponent.MaxWalkSpeed` (`KismetMathLibrary.FInterpTo` _maxwalkspeed (`self.Speed_Walk`) _returnvalue 10.0) _charactermovement)
            (else
              (set `CharacterMovementComponent.MaxWalkSpeed` (`KismetMathLibrary.FInterpTo` _maxwalkspeed (`self.Speed_Jog`) _returnvalue 10.0) _charactermovement))))))))

(event `Event_BattleStart`
  (bind _springarm (`self.SpringArm`))
  (bind (_returnvalue_roll _returnvalue_pitch) (`KismetMathLibrary.BreakRotator` (`SpringArmComponent.GetTargetRotation` _springarm)))
  ;[1 1 1] 전투 시작 시에 카메라를 캐릭터 뒤로 옮김
  (`SceneComponent.K2_SetWorldRotation` _springarm (`KismetMathLibrary.MakeRotator` _returnvalue_roll _returnvalue_pitch -90.0) false false)
  (set `SpringArmComponent.bUsePawnControlRotation` true (`self.SpringArm`)))

(event `self.ReceiveBeginPlay`
  ;[1 1 1] 시작
  (set `self.OriginArmLength` (`SpringArmComponent.TargetArmLength` (`self.SpringArm`)))
  ;;[1 1 1] 캐릭터 메시 결정
  (`SkinnedMeshComponent.SetSkinnedAssetAndUpdate` (`self.Mesh`) (`|GetArrayItem` (`self.MeshCharArray`) (`self.MeshCharIndex`)) true)
  ;;[1 1 1] 무기 장착
  (`self.ChangeWeapon` 0))

(event `Key|LeftControl`
  (params (Key :type "Key Structure"))
  ;[1 1 1] Walk
  (:`Pressed`
    (set `self.isWalk` true))
  (:`Released`
    (set `self.isWalk` false)))

(event `SnapRotation`
  ;[1 1 1] Snap Rotation
  (set `self.IsSnapRotation` true)
  (`KismetSystemLibrary.RetriggerableDelay` 0.2)
  (set `self.IsSnapRotation` false))

(event `Reset Attack`
  ;[1 1 1] Reset Attack
  (set `self.isAttack` false)
  (set `self.isAttack_Second` false))

(event `InputAction|Run`
  (params (Key :type "Key Structure"))
  ;[1 1 1] Run
  (:`Pressed`
    (set `self.isHoldShift` true)
    (if (< (`self.RunTimer`) 10)
      _))
  (:`Released`
    (set `self.isHoldShift` false)
    (set `self.pre_RunTimer` 0)
    (if (not (< (`self.RunTimer`) 10))
      (`KismetSystemLibrary.Delay` 0.15)
      (set `self.RunTimer` 0))))

(event `ResetDodge`
  ;[1 1 1] Reset Dodge
  (set `self.isDodge` false))

(event `ResetDamage`
  ;[1 1 1] Reset Damage
  (set `self.isDamage` false)
  (set `self.isDodge` false)
  (set `self.isAttack` false))

(event `InputAction|Dodge`
  (params (Key :type "Key Structure"))
  ;[1 1 1] 회피( 구르기 )
  (:`Pressed`
    (if (not (`self.isDodge`))
      (set `self.RunTimer` 0)
      (set `self.pre_RunTimer` 0)
      (set `self.inputVector` (`KismetMathLibrary.MakeVector` (`self.inputX_Local`) (`self.inputY_Local`)))
      (if (`NavMovementComponent.IsMovingOnGround` (`self.CharacterMovement`))
        (set `self.isDodge` true)))))

(event `InputAction|MB_Left`
  (params (Key :type "Key Structure"))
  ;[1 1 1] 드래그 + 마우스 회전⇾ 카메라 회전 (폐기)
)

(event `InputAxis|MoveForward`
  (params (AxisValue :type "Float (single-precision)"))
  (bind (_returnvalue_roll _returnvalue_pitch _returnvalue_yaw) (`KismetMathLibrary.BreakRotator` (`self.GetControlRotation`)))
  (bind _returnvalue (`KismetMathLibrary.MakeRotator` 0.0 0.0 _returnvalue_yaw))
  (bind _returnvalue_2 (`KismetMathLibrary.GetForwardVector` _returnvalue))
  ;[1 1 1] 캐릭터 앞, 뒤, 좌, 우 (W, S, A, D)
  (if (not (`self.OnCustomize`))
    (bind _output_get (set `self.inputY` AxisValue))
    (`self.AddMovementInput` _returnvalue_2 _output_get)
    (bind _returnvalue_3 (+ (* _returnvalue_2 _output_get) (* (`KismetMathLibrary.GetRightVector` _returnvalue) (stale `InputAxis|MoveRight` _output_get))))
    (set `self.inputVector_World` _returnvalue_3)
    (bind (_returnvalue_x _returnvalue_y) (`KismetMathLibrary.BreakVector` (`KismetMathLibrary.InverseTransformDirection` (`self.GetTransform`) _returnvalue_3)))
    (set `self.inputY_Local` _returnvalue_x)
    (set `self.inputX_Local` _returnvalue_y :!label _label)))

(event `Damage`
  (params (`Damage Position` :type "Vector Structure") (`Damage Type` :type Integer))
  (bind _returnvalue (- `Damage Position` (`self.K2_GetActorLocation`)))
  (bind (_returnvalue_roll _returnvalue_pitch _returnvalue_yaw) (`KismetMathLibrary.BreakRotator` (`KismetMathLibrary.Conv_VectorToRotator` (`KismetMathLibrary.Normal` _returnvalue))))
  ;[1 1 1] Damage
  (set `self.isDamage` true)
  (bind _output_get (set `self.DamageType` `Damage Type`))
  (`KismetSystemLibrary.PrintString` (`KismetStringLibrary.Concat_StrStr` "Damage Type : " (`KismetStringLibrary.Conv_IntToString` _output_get)))
  (set `self.DamagePosition` (`KismetMathLibrary.Normal` (`KismetMathLibrary.InverseTransformDirection` (`self.GetTransform`) _returnvalue)))
  (if (== (`self.DamageType`) 1)
    (`self.K2_SetActorRotation` (`KismetMathLibrary.MakeRotator` 0.0 0.0 _returnvalue_yaw) true)))

(event `InputAxis|Turn`
  (params (AxisValue :type "Float (single-precision)"))
  ;[1 1 1] 드래그 + 마우스 회전⇾ 카메라 회전 (폐기)
)

(event `InputAxis|MoveRight`
  (params (AxisValue :type "Float (single-precision)"))
  (bind (_returnvalue_roll _returnvalue_pitch _returnvalue_yaw) (`KismetMathLibrary.BreakRotator` (`self.GetControlRotation`)))
  ;[1 1 1] 캐릭터 앞, 뒤, 좌, 우 (W, S, A, D)
  (if (not (`self.OnCustomize`))
    (bind _output_get (set `self.inputX` AxisValue))
    (`self.AddMovementInput` (`KismetMathLibrary.GetRightVector` (`KismetMathLibrary.MakeRotator` 0.0 0.0 _returnvalue_yaw)) _output_get)
    (goto _label)))

(event `InputAxis|LookUp`
  (params (AxisValue :type "Float (single-precision)"))
  ;[1 1 1] 드래그 + 마우스 회전⇾ 카메라 회전 (폐기)
)

(event `InputAction|WheelUp`
  (params (Key :type "Key Structure"))
  ;[1 1 1] 확대, 축소
  (:`Pressed`
    (bind _output_get (set `self.OriginArmLength` (- (`self.OriginArmLength`) 20.0)))
    (if (< _output_get 50.0)
      (set `self.OriginArmLength` 50.0))))

(event `InputAction|WheelDown`
  (params (Key :type "Key Structure"))
  ;[1 1 1] 확대, 축소
  (:`Pressed`
    (bind _output_get (set `self.OriginArmLength` (+ (`self.OriginArmLength`) 20.0)))
    (if (> _output_get 400.0)
      (set `self.OriginArmLength` 400.0))))

(event `Key|E`
  (params (Key :type "Key Structure"))
  (bind (_information_hp _information_strength _information_agility _information_stemina) (break `/Game/Blueprint/Character/PlayerStruct` (`self.Information`)))
  (:`Pressed`
    (set `self.Information` (make `/Game/Blueprint/Character/PlayerStruct` (- _information_hp 10.0) _information_strength _information_agility _information_stemina))))

(event `InputAction|MB_Left`
  (params (Key :type "Key Structure"))
  (bind _oncustomize (`self.OnCustomize`))
  ;[1 1 1] 드래그 + 마우스 X 회전 = 캐릭터 회전
  (:`Pressed`
    (if _oncustomize
      (set `self.MB_Left_Press` true)
      (else
        ;;[1 1 1] Attack
        (set `self.isAttack` true))))
  (:`Released`
    (if _oncustomize
      (set `self.MB_Left_Press` false)
      (else
        (set `self.isAttack` false)
        (set `self.isAttack_Second` false :!label _label_2)))))

(event `Key|F`
  (params (Key :type "Key Structure"))
  (bind (_information_hp _information_strength _information_agility _information_stemina) (break `/Game/Blueprint/Character/PlayerStruct` (`self.Information`)))
  (:`Pressed`
    (set `self.Information` (make `/Game/Blueprint/Character/PlayerStruct` _information_hp _information_strength _information_agility (- _information_stemina 10.0)))))

(event `InputAction|MB_Right`
  (params (Key :type "Key Structure"))
  (bind _oncustomize (`self.OnCustomize`))
  ;[1 1 1] 드래그 + 마우스 X 회전 = 캐릭터 회전
  (:`Pressed`
    (if (not _oncustomize)
      ;;[1 1 1] Attack
      (set `self.isAttack_Second` true)))
  (:`Released`
    (if (not _oncustomize)
      (goto _label_2))))

(event `InputAxis|Turn`
  (params (AxisValue :type "Float (single-precision)"))
  (bind _mesh (`self.Mesh`))
  (bind (_returnvalue_roll _returnvalue_pitch _returnvalue_yaw) (`KismetMathLibrary.BreakRotator` (`SceneComponent.K2_GetComponentRotation` _mesh)))
  ;[1 1 1] 드래그 + 마우스 X 회전 = 캐릭터 회전
  (if (`self.OnCustomize`)
    (if (`self.MB_Left_Press`)
      (`SceneComponent.K2_SetWorldRotation` _mesh (`KismetMathLibrary.MakeRotator` _returnvalue_roll _returnvalue_pitch (+ (* AxisValue 0.25) _returnvalue_yaw)) false false))
    (else
      ;;[1 1 1] 캐릭터 회전
      (`self.AddControllerYawInput` AxisValue))))

(event `InputAxis|LookUp`
  (params (AxisValue :type "Float (single-precision)"))
  ;[1 1 1] 드래그 + 마우스 X 회전 = 캐릭터 회전
  ;;[1 1 1] 캐릭터 회전
  (if (not (`self.OnCustomize`))
    (`self.AddControllerPitchInput` AxisValue)))

(event `Key|Right`
  (params (Key :type "Key Structure"))
  ;[1 1 1] 캐릭터 매쉬 변경 (임시) (뱡향키 좌우 클릭)
  (:`Pressed`
    (bind _result (`/Engine/EditorBlueprintResources/StandardMacros.IncrementInt` (`self.MeshCharIndex`))
      (:`  `
        (if (> _result (`KismetArrayLibrary.Array_LastIndex` (`self.MeshCharArray`)))
          (set `self.MeshCharIndex` 0))
        (`SkinnedMeshComponent.SetSkinnedAssetAndUpdate` (`self.Mesh`) (`|GetArrayItem` (`self.MeshCharArray`) (`self.MeshCharIndex`)) true)))))

(event `Key|Left`
  (params (Key :type "Key Structure"))
  ;[1 1 1] 캐릭터 매쉬 변경 (임시) (뱡향키 좌우 클릭)
  (:`Pressed`
    (bind _result (`/Engine/EditorBlueprintResources/StandardMacros.DecrementInt` (`self.MeshCharIndex`))
      (:`  `
        (if (< _result 0)
          (set `self.MeshCharIndex` (`KismetArrayLibrary.Array_LastIndex` (`self.MeshCharArray`))))
        (`SkinnedMeshComponent.SetSkinnedAssetAndUpdate` (`self.Mesh`) (`|GetArrayItem` (`self.MeshCharArray`) (`self.MeshCharIndex`)) true)))))

(fn `AngleRange`
  (params (Min :type "Float (double-precision)") (Max :type "Float (double-precision)") (angle :type "Float (double-precision)"))
  (returns (NewParam1 :type Boolean))
  (if (<= Min angle)
    (if (>= Max angle)
      (return true)
      (else
        _)))
  (return false))

(fn `ChangeWeapon`
  (params (index :type Integer))
  (bind _swordsocket (`self.SwordSocket`))
  (bind _equipselect (`self.EquipSelect`))
  (bind _shieldsocket (`self.ShieldSocket`))
  (set `self.EquipSelect` index)
  ;[1 1 1] 기본 무기 (임시 양손검 고정)
  (`StaticMeshComponent.SetStaticMesh` _swordsocket (`|GetArrayItem` (`self.WeaponStack`) _equipselect))
  (`SceneComponent.K2_SetRelativeTransform` _swordsocket (`|GetArrayItem` (`self.WeaponTransform`) _equipselect) false false)
  ;[1 1 1] 방패
  (`StaticMeshComponent.SetStaticMesh` _shieldsocket (`|GetArrayItem` (`self.ShieldStack`) _equipselect))
  (`SceneComponent.K2_SetRelativeTransform` _shieldsocket (`|GetArrayItem` (`self.ShieldTransform`) _equipselect) false false))

(fn `UserConstructionScript`)