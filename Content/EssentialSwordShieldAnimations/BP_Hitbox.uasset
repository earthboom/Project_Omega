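; BP_Hitbox is an actor that triggers a hurt response on any BP_ThirdPersonCharacter that overlaps it.
; It calls the character's Hurt with its own location and AttackType, then disables collision and hides the Hitbox component.
; About two seconds later it shows the component again and re-enables collision shortly after, so it can hit repeatedly.
; The construction script picks a light or heavy material from AttackType.
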(event `self.ReceiveActorBeginOverlap`
  (params (OtherActor :type "Actor Object Reference"))
  (bind _asthird_person_character (cast `/Game/EssentialSwordShieldAnimations/BP_ThirdPersonCharacter` OtherActor))
  (`/Game/EssentialSwordShieldAnimations/BP_ThirdPersonCharacter.Hurt` _asthird_person_character (`self.K2_GetActorLocation`) (`self.AttackType`))
  (`KismetSystemLibrary.PrintString` "Hit")
  (`self.SetActorEnableCollision` false)
  (`SceneComponent.SetVisibility` (`self.Hitbox`) false false)
  (`KismetSystemLibrary.Delay` 2.0)
  (`SceneComponent.SetVisibility` (`self.Hitbox`) true false)
  (`KismetSystemLibrary.Delay` 0.1)
  (`self.SetActorEnableCollision` true))

(fn `UserConstructionScript`
  (bind _hitbox (`self.Hitbox`))
  (if (== (`self.AttackType`) 0)
    (`PrimitiveComponent.SetMaterial` _hitbox 0 "/Game/EssentialSwordShieldAnimations/Material/MI_Hitbox_Light.MI_Hitbox_Light")
    (else
      (`PrimitiveComponent.SetMaterial` _hitbox 0 "/Game/EssentialSwordShieldAnimations/Material/MI_Hitbox_Heavy.MI_Hitbox_Heavy"))))